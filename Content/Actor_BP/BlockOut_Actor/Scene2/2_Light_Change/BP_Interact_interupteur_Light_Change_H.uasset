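; One-shot interactable light switch for Scene 2 that changes the lighting and shadow setup.
; On its first Interact, it briefly shows the On_Light1 widget while destroying the referenced light and spawning a Mecha_Shadow_Spawn at the configured location and scale.
; It also finds the BP_Interact_interupteur_Light_Change_S switch and clears its InterupteurShadow flag.
; Short delays stagger the swap and the widget's removal.
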(event EventBeginPlay)

(event Collision|EventActorBeginOverlap
  (params (OtherActor :type Actor%20Object%20Reference)))

(event EventTick
  (params (DeltaSeconds :type Float%20%28single-precision%29)))

(event EventInteract
  (params (Humain :type BP%20Humain%20Object%20Reference) (Shadow :type BP%20Shadow%20Object%20Reference))
  (Utilities|FlowControl|DoOnce false
    (:Completed
      (bind _returnvalue (UserInterface|CreateWidget "/Game/Actor_BP/Widget/On_Light1.On_Light1_C"))
      (UserInterface|Viewport|AddtoViewport _returnvalue 0)
      (Utilities|FlowControl|Delay 0.1)
      (Actor|DestroyActor (Variables|Default|GetLight%20Destroy))
      (Game|SpawnActorfromClass "/Game/Actor_BP/BlockOut_Actor/Scene2/1_Light_Spawn/Mecha_Shadow_Spawn.Mecha_Shadow_Spawn_C" (Math|Transform|MakeTransform (Variables|Default|GetShadow%20New%20Location) "0, 0, 0" (Variables|Default|GetShadow%20New%20Scale)) "Undefined" 0 0)
      (bind _returnvalue_2 (Actor|GetActorOfClass "/Game/Actor_BP/BlockOut_Actor/Scene2/2_Light_Change/BP_Interact_interupteur_Light_Change_S.BP_Interact_interupteur_Light_Change_S_C"))
      (Variables|/Game/Actor_BP/BlockOut_Actor/Scene2/2_Light_Change/BP_Interact_interupteur_Light_Change_S.BP_Interact_interupteur_Light_Change_S_C|SetInterupteur%20Shadow%20? _returnvalue_2 false)
      (Utilities|FlowControl|Delay 0.4)
      (Widget|RemovefromParent _returnvalue))))

(fn ConstructionScript)